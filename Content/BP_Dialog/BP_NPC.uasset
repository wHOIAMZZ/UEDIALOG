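; NPC Blueprint that opens a dialog UI when interacted with.
; Interact creates a UMG_DIALOG widget from the NPC's DialogTable, binds DialogEnd to it, adds it to the viewport and switches player 0 to UI-only input with a visible cursor.
; DialogEnd removes the widget, restores game-only input and hides the cursor.
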(event `self.Interact`
  (bind _returnvalue (`GameplayStatics.GetPlayerController` 0))
  (bind _returnvalue_2 (`|CreateWidget` "/Game/BP_Dialog/UMG_DIALOG.UMG_DIALOG_C" null (`self.DialogTable`)))
  (bind _output_get (set `self.Dialog Widget` _returnvalue_2))
  (add `/Game/BP_Dialog/UMG_DIALOG.DialogEnd` _output_get (delegate `DialogEnd`))
  (`UserWidget.AddToViewport` _output_get 0)
  (`WidgetBlueprintLibrary.SetInputMode_UIOnlyEx` _returnvalue null)
  (set `PlayerController.bShowMouseCursor` true _returnvalue))

(event `DialogEnd`
  (bind _returnvalue (`GameplayStatics.GetPlayerController` 0))
  (`Widget.RemoveFromParent` (`self.Dialog Widget`))
  (`WidgetBlueprintLibrary.SetInputMode_GameOnly` _returnvalue)
  (set `PlayerController.bShowMouseCursor` false _returnvalue))

(fn `UserConstructionScript`
  (`parent.UserConstructionScript`))